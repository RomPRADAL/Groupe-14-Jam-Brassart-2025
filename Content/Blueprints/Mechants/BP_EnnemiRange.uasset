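; BP_EnnemiRange is an enemy, voiced with Nutcracker sounds, that loses health when hit by projectiles and dies at zero.
; A BP_Projectile overlapping the capsule passes its damage to TakeDmg and triggers a hurt sound.
; TakeDmg lowers Health and calls CheckDeath; Death then spawns a Niagara effect, plays a death sound and destroys the actor.
; Debug prints show health and death, and no attack or movement logic is present in these graphs.
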(event OnComponentBeginOverlap(StaticMesh)
  (params (OverlappedComponent :type Primitive%20Component%20Object%20Reference) (OtherActor :type Actor%20Object%20Reference) (OtherComp :type Primitive%20Component%20Object%20Reference) (OtherBodyIndex :type Integer) (bFromSweep :type Boolean) (SweepResult :type Hit%20Result%20Structure%20%28by%20ref%29)))

(event OnComponentBeginOverlap(CapsuleComponent)
  (params (OverlappedComponent :type Primitive%20Component%20Object%20Reference) (OtherActor :type Actor%20Object%20Reference) (OtherComp :type Primitive%20Component%20Object%20Reference) (OtherBodyIndex :type Integer) (bFromSweep :type Boolean) (SweepResult :type Hit%20Result%20Structure%20%28by%20ref%29))
  (bind _asbp_projectile (Utilities|Casting|CastToBP_Projectile OtherActor))
  (CallFunction|TakeDmg (Variables|/Game/Blueprints/Flingues/BP_Projectile.BP_Projectile_C|GetDmg _asbp_projectile))
  (Audio|PlaySound2D "/Game/Sounds/NutcrackerDamaged.NutcrackerDamaged" 1.0 1.0 0.0 0 0))

(event EventBeginPlay)

(event Collision|EventActorBeginOverlap
  (params (OtherActor :type Actor%20Object%20Reference)))

(event EventTick
  (params (DeltaSeconds :type Float%20%28single-precision%29)))

(fn ConstructionScript)

(fn Death
  (Development|PrintString "T'es mort hihi" true true "(R=1.000000,G=0.061336,B=0.041440,A=1.000000)")
  (Niagara|SpawnSystematLocation "/Game/Blueprints/Flingues/Niagara_EnnemyDeath.Niagara_EnnemyDeath" (Transformation|GetWorldLocation (Variables|Character|GetMesh)))
  (Audio|PlaySound2D "/Game/Sounds/NutcrakerDeath.NutcrakerDeath" 1.0 1.0 0.0 0 0)
  (Actor|DestroyActor))

(fn CheckDeath
  (if (<= (Variables|Default|GetHealth) 0.0)
    (LocalVariables|SetRetDead true))
  (return (LocalVariables|GetRetDead)))

(fn TakeDmg
  (params (Dmg :type Float%20%28double-precision%29))
  (bind _output_get (Variables|Default|SetHealth (- (Variables|Default|GetHealth) Dmg)))
  (Development|PrintString (Utilities|String|ToString(Float) _output_get) true true "(R=0.141462,G=1.000000,B=0.490336,A=1.000000)")
  (bind _dead_ (CallFunction|CheckDeath))
  (if _dead_
    (CallFunction|Death)))