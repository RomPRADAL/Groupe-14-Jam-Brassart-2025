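; BoutonTuto is a tutorial button actor that opens the tutorial door when hit by a projectile.
; On BeginPlay it finds a PorteTuto actor in the level with GetActorOfClass and caches it.
; When a BP_Projectile begins overlapping its Box, it calls OpenDodoor on that door if the reference is valid.
; An unconnected cast to GI_Doudoom remains in the graph and never runs.
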(event OnComponentBeginOverlap(Box)
  (params (OverlappedComponent :type Primitive%20Component%20Object%20Reference) (OtherActor :type Actor%20Object%20Reference) (OtherComp :type Primitive%20Component%20Object%20Reference) (OtherBodyIndex :type Integer) (bFromSweep :type Boolean) (SweepResult :type Hit%20Result%20Structure%20%28by%20ref%29))
  (Utilities|Casting|CastToBP_Projectile OtherActor)
  (Utilities|IsValid (Variables|Default|GetDodoor)
    (:Is%20Valid
      (Default|OpenDodoor (Variables|Default|GetDodoor)))))

(event EventBeginPlay
  (bind _returnvalue (Actor|GetActorOfClass "/Game/Blueprints/Portes/PorteTuto.PorteTuto_C"))
  (Variables|Default|SetDodoor _returnvalue))

(event Collision|EventActorBeginOverlap
  (params (OtherActor :type Actor%20Object%20Reference)))

(event EventTick
  (params (DeltaSeconds :type Float%20%28single-precision%29)))

(fn ConstructionScript)